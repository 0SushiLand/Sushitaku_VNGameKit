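; String function library that prepares raw text for display by cleaning markup and filling in variables.
; ConvertCleanText trims the text, collapses line-break codes adjacent to next-page tags, converts remaining line-break codes, then passes the result to ConvertVariable.
; ConvertVariable regex-extracts brace-wrapped names and replaces each with its status value from BP_GameInstance.
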(fn ConvertCleanText
  (params (Text :type String))
  (bind _asbp_game_instance (Utilities|Casting|CastToBP_GameInstance (Game|GetGameInstance)))
  (LocalVariables|SetGameInstance _asbp_game_instance)
  (return (CallFunction|ConvertVariable (Utilities|String|Replace (Utilities|String|Replace (Utilities|String|Replace (Utilities|String|Trim Text) (Utilities|String|Append (LocalVariables|GetTagNextPage) (LocalVariables|GetIndention)) (LocalVariables|GetTagNextPage)) (Utilities|String|Append (LocalVariables|GetIndention) (LocalVariables|GetTagNextPage)) (LocalVariables|GetTagNextPage)) (LocalVariables|GetIndention) " 
"))))

(fn ConvertVariable
  (params (Text :type String))
  (LocalVariables|SetReturnText Text)
  (bind _asbp_game_instance (Utilities|Casting|CastToBP_GameInstance (Game|GetGameInstance)))
  ;[0.15 0.15 0.15 0.5] 変数名を値に変換
  (for _array_element (Class|Utility|ExtractPattern Text "\\{(.*?)\\}" false)
    (LocalVariables|SetReturnText (Utilities|String|Replace (LocalVariables|GetReturnText) (Utilities|String|Append "{" _array_element "}") (.Value (Default|GetStatus _asbp_game_instance _array_element)))))
  (return (LocalVariables|GetReturnText)))
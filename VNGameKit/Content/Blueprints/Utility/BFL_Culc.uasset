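; Function library for dice-notation rolls and numeric comparisons.
; RollDice regex-extracts XdY terms, rolls them, and returns cleaned detail text with bracketed rolls plus a truncated total from EvaluateExpression.
; Its expression substitution sits inside the summing loop, so each term takes only its first die's value.
; CheckComparison maps an operator, including = and <>, to a boolean comparison of Left and Right.
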(fn RollDice
  (params (Text :type String))
  (bind _output_get (LocalVariables|SetReturnDetail Text))
  (LocalVariables|SetExpr _output_get)
  (for _array_element (Class|Utility|ExtractPattern Text "(\\d+)[dD](\\d+)" true)
    (bind _output_get_2 (LocalVariables|SetDice _array_element))
    (Utilities|FlowControl|Sequence
      (:then_0
        ;[0.15 0.15 0.15 0.5] ダイスロール
        (Utilities|Array|Clear (LocalVariables|GetRollResult))
        (LocalVariables|SetDiceNum (Math|Conversions|ToInteger(Byte) (Utilities|Array|Get(acopy) (Utilities|String|ParseIntoArray _output_get_2 "d"))))
        (LocalVariables|SetMax (Math|Conversions|ToInteger(Byte) (Utilities|Array|Get(acopy) (Utilities|String|ParseIntoArray _output_get_2 "d") 1)))
        (for _index (range 0 (- (LocalVariables|GetDiceNum) 1))
          (LocalVariables|SetRandomInt (Math|Random|RandomIntegerinRange 1 (LocalVariables|GetMax)))
          (Utilities|Array|Add (LocalVariables|GetRollResult) (Utilities|String|ToString(Integer) (LocalVariables|GetRandomInt)))))
      (:then_1
        ;[0.15 0.15 0.15 0.5] 結果表示用
        (LocalVariables|SetRollText "")
        (LocalVariables|SetRollText (Utilities|String|Append "[" (Utilities|String|JoinStringArray (LocalVariables|GetRollResult) ",") "]"))
        (LocalVariables|SetReturnDetail (Utilities|String|Replace (LocalVariables|GetReturnDetail) (LocalVariables|GetDice) (LocalVariables|GetRollText))))
      (:then_2
        ;[0.15 0.15 0.15 0.5] 計算用
        (LocalVariables|SetRollSum "0")
        (for _array_element_2 (LocalVariables|GetRollResult)
          (LocalVariables|SetRollSum (Utilities|String|ToString(Integer) (+ (Math|Conversions|ToInteger(Byte) (LocalVariables|GetRollSum)) (Math|Conversions|ToInteger(Byte) _array_element_2))))
          (LocalVariables|SetExpr (Utilities|String|Replace (LocalVariables|GetExpr) (LocalVariables|GetDice) (LocalVariables|GetRollSum)))))))
  ;[0.15 0.15 0.15 0.5] 合計値
  (LocalVariables|SetReturnResult (Math|Float|Truncate (Class|Utility|EvaluateExpression (CallFunction|ConvertCleanText (LocalVariables|GetExpr)))))
  (return (CallFunction|ConvertCleanText (LocalVariables|GetReturnDetail)) (LocalVariables|GetReturnResult)))

(fn CheckComparison
  (params (Left :type Integer) (condition :type String) (Right :type Integer))
  ;[0.15 0.15 0.15 0.5] 比較
  (switch string condition
    (:>=
      (return (>= Left Right)))
    (:<=
      (return (<= Left Right)))
    (:==
      (return (== Left Right)))
    (:<>
      (return (!= Left Right)))
    (:>
      (return (> Left Right)))
    (:<
      (return (< Left Right)))
    (:=
      (return (== Left Right)))))